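; BP_TDRL_HUD is the HUD for the TDRL game, owning the in-game UI widget and relaying weapon slot, icon and grenade updates to it.
; CreateinGameUI spawns WBP_TDRL_InGameUI once for player 0, passes itself as HUDReference and adds it to the viewport.
; Overridden slot, selection, icon, ammo and grenade events call the parent version, then forward to the widget if it is valid.
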(event `self.CreateInGameUI`
  (`/Engine/EditorBlueprintResources/StandardMacros.IsValid` (`self.InGameRef`)
    (:`Is Not Valid`
      (bind _returnvalue (`|CreateWidget` "/TopDownRogueLite/TDRL/Blueprints/HUD/WBP_TDRL_InGameUI.WBP_TDRL_InGameUI_C" (`GameplayStatics.GetPlayerController` 0) self))
      (bind _output_get (set `self.InGameRef` _returnvalue))
      (`UserWidget.AddToViewport` _output_get 0))))

(event `self.SetSlotsAmount`
  (params (Slot :type Byte))
  (`parent.SetSlotsAmount` Slot)
  (bind _ingameref (`self.InGameRef`)
    (:`then`
      (`/TopDownRogueLite/TDRL/Blueprints/HUD/WBP_TDRL_InGameUI.SetSlotsAmount` _ingameref Slot))
    (:`else`)))

(event `self.SelectSlotUI`
  (params (Slot :type Byte))
  (`parent.SelectSlotUI` Slot)
  (bind _ingameref (`self.InGameRef`)
    (:`then`
      (`/TopDownRogueLite/TDRL/Blueprints/HUD/WBP_TDRL_InGameUI.SelectSlot` _ingameref Slot))
    (:`else`)))

(event `self.RefreshIcons`
  (`parent.RefreshIcons`)
  (bind _ingameref (`self.InGameRef`)
    (:`then`
      (`/TopDownRogueLite/TDRL/Blueprints/HUD/WBP_TDRL_InGameUI.RefreshIcons` _ingameref))
    (:`else`)))

(event `self.RefreshAmmoSlot`
  (params (Slot :type Byte))
  (`parent.RefreshAmmoSlot` Slot)
  (bind _ingameref (`self.InGameRef`)
    (:`then`
      (`/TopDownRogueLite/TDRL/Blueprints/HUD/WBP_TDRL_InGameUI.RefreshAmmoSlot` _ingameref Slot))
    (:`else`)))

(event `self.RefreshGrenadeWidget`
  (`parent.RefreshGrenadeWidget`)
  (bind _ingameref (`self.InGameRef`)
    (:`then`
      (`/TopDownRogueLite/TDRL/Blueprints/HUD/WBP_TDRL_InGameUI.RefreshGrenadeWidget` _ingameref))
    (:`else`)))

(fn `UserConstructionScript`)