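; GA_PrimaryAction is an input-driven Gameplay Ability that starts and stops a TDRL_Character's primary action.
; On activation it cancels if the owner is not a TDRL_Character or is stunned; otherwise it begins the action and waits for input release to end.
; OnEndAbility always tells the owning character to stop the primary action, so the action lasts while the input is held.
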(event `self.K2_ActivateAbility`
  (bind _returnvalue_owneractor (break `GameplayAbilityActorInfo` (`self.GetActorInfo`)))
  (bind _astdrl_character (cast `TDRL_Character` _returnvalue_owneractor)
    (:`then`
      (if (`TDRL_Character.IsStunned` _astdrl_character)
        (`self.K2_CancelAbility`)
        (else
          (`TDRL_Character.PerformPrimaryAction` _astdrl_character true)
          (`AbilityTask_WaitInputRelease.WaitInputRelease` false
            (:`OnRelease`
              (`self.K2_EndAbility`))))))
    (:`CastFailed`
      (`self.K2_CancelAbility`))))

(event `self.K2_OnEndAbility`
  (params (bWasCancelled :type Boolean))
  (bind _returnvalue_owneractor (break `GameplayAbilityActorInfo` (`self.GetActorInfo`)))
  (bind _astdrl_character (cast `TDRL_Character` _returnvalue_owneractor))
  (`TDRL_Character.PerformPrimaryAction` _astdrl_character false))