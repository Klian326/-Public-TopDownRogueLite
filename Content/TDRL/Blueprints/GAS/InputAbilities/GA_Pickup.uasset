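; GA_Pickup is a Gameplay Ability, filed with the input abilities, that lets a TDRL character pick up the nearest nearby item.
; On activation it casts the owner actor to TDRL_Character, then cancels if the cast fails, the character is stunned or no valid item is nearby.
; Otherwise it passes that item to the character's PickupItem and ends immediately, leaving item detection and pickup logic to the character.
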(event `self.K2_ActivateAbility`
  (bind _returnvalue_owneractor (break `GameplayAbilityActorInfo` (`self.GetActorInfo`)))
  (bind _astdrl_character (cast `TDRL_Character` _returnvalue_owneractor)
    (:`then`
      (if (`TDRL_Character.IsStunned` _astdrl_character)
        (`self.K2_CancelAbility`)
        (else
          (bind _returnvalue (`TDRL_Character.GetNearestNearbyItem` _astdrl_character))
          (`/Engine/EditorBlueprintResources/StandardMacros.IsValid` _returnvalue
            (:`Is Valid`
              (`TDRL_Character.PickupItem` _astdrl_character _returnvalue)
              (`self.K2_EndAbility`))
            (:`Is Not Valid`
              (`self.K2_CancelAbility`))))))
    (:`CastFailed`
      (`self.K2_CancelAbility`))))

(event `self.K2_OnEndAbility`
  (params (bWasCancelled :type Boolean)))