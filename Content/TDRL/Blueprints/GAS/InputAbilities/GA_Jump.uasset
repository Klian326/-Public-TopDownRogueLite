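; GA_Jump is a Gameplay Ability that handles the player's jump input for TDRL_Character.
; Activation cancels if the owner is not a TDRL_Character or is stunned, and uncrouches and ends immediately if crouching.
; Otherwise it calls Jump and waits for input release to end, with OnEndAbility calling StopJumping so hold duration controls the jump.
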(event `self.K2_ActivateAbility`
  (bind _returnvalue_owneractor (break `GameplayAbilityActorInfo` (`self.GetActorInfo`)))
  (bind _astdrl_character (cast `TDRL_Character` _returnvalue_owneractor)
    (:`then`
      (if (`TDRL_Character.IsStunned` _astdrl_character)
        (`self.K2_CancelAbility`)
        (elif (`NavMovementComponent.IsCrouching` (`Character.CharacterMovement` _astdrl_character))
          (`Character.UnCrouch` _astdrl_character)
          (`self.K2_EndAbility`)
          (else
            (`Character.Jump` _astdrl_character)
            (`AbilityTask_WaitInputRelease.WaitInputRelease` false
              (:`OnRelease`
                (`self.K2_EndAbility`)))))))
    (:`CastFailed`
      (`self.K2_CancelAbility`))))

(event `self.K2_OnEndAbility`
  (params (bWasCancelled :type Boolean))
  (bind _returnvalue_owneractor (break `GameplayAbilityActorInfo` (`self.GetActorInfo`)))
  (bind _ascharacter (cast `Character` _returnvalue_owneractor))
  (`Character.StopJumping` _ascharacter))