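; GA_Crouch is a Gameplay Ability that toggles crouch on the owning TDRL_Character.
; On activation it uncrouches the character if already crouching, or crouches it if not falling, then ends immediately.
; It cancels instead when the owner cast fails, the character is stunned, or a crouch is attempted while falling.
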(event `self.K2_ActivateAbility`
  (bind _returnvalue_owneractor (break `GameplayAbilityActorInfo` (`self.GetActorInfo`)))
  (bind _astdrl_character (cast `TDRL_Character` _returnvalue_owneractor)
    (:`then`
      (if (`TDRL_Character.IsStunned` _astdrl_character)
        (`self.K2_CancelAbility`)
        (else
          (bind _charactermovement (`Character.CharacterMovement` _astdrl_character))
          (if (`NavMovementComponent.IsCrouching` _charactermovement)
            (`Character.UnCrouch` _astdrl_character)
            (`self.K2_EndAbility`)
            (elif (not (`NavMovementComponent.IsFalling` _charactermovement))
              (`Character.Crouch` _astdrl_character)
              (`self.K2_EndAbility`)
              (else
                (`self.K2_CancelAbility`)))))))
    (:`CastFailed`
      (`self.K2_CancelAbility`))))

(event `self.K2_OnEndAbility`
  (params (bWasCancelled :type Boolean)))