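; Player controller for the top-down TDRL game that forwards Enhanced Input actions to the possessed TDRL character.
; It aims by switching control rotation between a mouse Z-plane mode, shown by a Niagara beam cursor, and a locked-target mode.
; Lock-on picks the nearest character under the mouse, hides the cursor and clears when that target dies.
; It also moves the cursor by thumbstick and respawns the player at the last valid start tag.
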(event `self.ReceiveTick`
  (params (DeltaSeconds :type "Float (single-precision)"))
  (bind _niagaracursor (`self.NiagaraCursor`))
  ;[1 1 1] Cursor indicator
  (`|ExecutionSequence`
    (:`then_0`
      (`/Engine/EditorBlueprintResources/StandardMacros.IsValid` _niagaracursor
        (:`Is Valid`
          (`SceneComponent.K2_SetWorldLocation` _niagaracursor (`self.ZPlaneTargetLocation`) false true)
          (`FXSystemComponent.SetVectorParameter` (`self.NiagaraCursor`) "BeamEnd" (- (`self.ZPlaneTargetLocation`) (`KismetMathLibrary.MakeVector` 0.0 0.0 (`self.ZPlaneFloorHeight`)))))))
    (:`then_1`)))

(event `self.ReceiveBeginPlay`
  (bind _returnvalue (subsystem `EnhancedInputLocalPlayerSubsystem`))
  (bind _returnvalue_2 (`NiagaraFunctionLibrary.SpawnSystemAtLocation` "/TopDownRogueLite/TDRL/DemoAssets/Niagara/NS_Cursor.NS_Cursor" (0.0 0.0 0.0) (struct) (1.0 1.0 1.0) false))
  (set `self.NiagaraCursor` _returnvalue_2)
  ;[1 1 1] Get focus of game's window without clicking it
  (`WidgetBlueprintLibrary.SetFocusToGameViewport`)
  ;[1 1 1] InputMode
  (`WidgetBlueprintLibrary.SetInputMode_GameAndUIEx` self null "LockAlways" false)
  ;[0.05098 0.05098 0.05098] Add Mapping Context
  (`/Engine/EditorBlueprintResources/StandardMacros.IsValid` _returnvalue
    (:`Is Valid`
      (`EnhancedInputSubsystemInterface.AddMappingContext` _returnvalue "/TopDownRogueLite/TDRL/Blueprints/Input/IMC_Default.IMC_Default" 0 (struct))
      ;[1 0 0] Control Rotation Type
      (`self.SetControlRotationType` "ZPlane"))))

(event `EnhancedInput|/TopDownRogueLite/TDRL/Blueprints/Input/Actions/Move`
  (params (ActionValue :type "Vector2D Structure") (ElapsedSeconds :type "Float (double-precision)") (TriggeredSeconds :type "Float (double-precision)") (InputAction :type "InputAction Object Reference" :default "/TopDownRogueLite/TDRL/Blueprints/Input/Actions/Move.Move"))
  (bind (_x _y) (`KismetMathLibrary.BreakVector2D` ActionValue))
  ;[1 1 1] Inputs
  (:`Triggered`
    (bind _possessedtdrlcharacter (`self.PossessedTDRLCharacter`)
      (:`then`
        (`TDRL_Character.Input_Move` _possessedtdrlcharacter (`KismetMathLibrary.MakeVector` _y _x)))
      (:`else`))))

(event `EnhancedInput|/TopDownRogueLite/TDRL/Blueprints/Input/Actions/SelectItemSlot_0`
  (params (ActionValue :type "Float (double-precision)") (ElapsedSeconds :type "Float (double-precision)") (TriggeredSeconds :type "Float (double-precision)") (InputAction :type "InputAction Object Reference" :default "/TopDownRogueLite/TDRL/Blueprints/Input/Actions/SelectItemSlot_0.SelectItemSlot_0"))
  ;[1 1 1] Inputs
  (:`Started`
    (bind _possessedtdrlcharacter (`self.PossessedTDRLCharacter`)
      (:`then`
        (`TDRL_Character.Input_ChangeItemSlot` _possessedtdrlcharacter (`KismetMathLibrary.Conv_IntToByte` (`KismetMathLibrary.Round` ActionValue))))
      (:`else`))))

(event `EnhancedInput|/TopDownRogueLite/TDRL/Blueprints/Input/Actions/RotateCamera`
  (params (ActionValue :type "Float (double-precision)") (ElapsedSeconds :type "Float (double-precision)") (TriggeredSeconds :type "Float (double-precision)") (InputAction :type "InputAction Object Reference" :default "/TopDownRogueLite/TDRL/Blueprints/Input/Actions/RotateCamera.RotateCamera"))
  ;[1 1 1] Inputs
  (:`Triggered`
    (bind _possessedtdrlcharacter (`self.PossessedTDRLCharacter`)
      (:`then`
        (`TDRL_Character.Input_RotateCamera` _possessedtdrlcharacter ActionValue))
      (:`else`))))

(event `EnhancedInput|/TopDownRogueLite/TDRL/Blueprints/Input/Actions/Interact`
  (params (ActionValue :type Boolean) (ElapsedSeconds :type "Float (double-precision)") (TriggeredSeconds :type "Float (double-precision)") (InputAction :type "InputAction Object Reference" :default "/TopDownRogueLite/TDRL/Blueprints/Input/Actions/Interact.Interact"))
  ;[1 1 1] Inputs
  (:`Started`
    (bind _possessedtdrlcharacter (`self.PossessedTDRLCharacter`)
      (:`then`
        (`TDRL_Character.Input_Interact` _possessedtdrlcharacter ActionValue))
      (:`else`))))

(event `EnhancedInput|/TopDownRogueLite/TDRL/Blueprints/Input/Actions/Jump`
  (params (ActionValue :type Boolean) (ElapsedSeconds :type "Float (double-precision)") (TriggeredSeconds :type "Float (double-precision)") (InputAction :type "InputAction Object Reference" :default "/TopDownRogueLite/TDRL/Blueprints/Input/Actions/Jump.Jump"))
  ;[1 1 1] Inputs
  (:`Started`
    (bind _possessedtdrlcharacter (`self.PossessedTDRLCharacter` :!label _label)
      (:`then`
        (`TDRL_Character.Input_Jump` _possessedtdrlcharacter ActionValue))
      (:`else`)))
  (:`Canceled`
    (goto _label))
  (:`Completed`
    (goto _label)))

(event `EnhancedInput|/TopDownRogueLite/TDRL/Blueprints/Input/Actions/Drop`
  (params (ActionValue :type Boolean) (ElapsedSeconds :type "Float (double-precision)") (TriggeredSeconds :type "Float (double-precision)") (InputAction :type "InputAction Object Reference" :default "/TopDownRogueLite/TDRL/Blueprints/Input/Actions/Drop.Drop"))
  ;[1 1 1] Inputs
  (:`Started`
    (bind _possessedtdrlcharacter (`self.PossessedTDRLCharacter`)
      (:`then`
        (`TDRL_Character.Input_Drop` _possessedtdrlcharacter ActionValue))
      (:`else`))))

(event `EnhancedInput|/TopDownRogueLite/TDRL/Blueprints/Input/Actions/Crouch`
  (params (ActionValue :type Boolean) (ElapsedSeconds :type "Float (double-precision)") (TriggeredSeconds :type "Float (double-precision)") (InputAction :type "InputAction Object Reference" :default "/TopDownRogueLite/TDRL/Blueprints/Input/Actions/Crouch.Crouch"))
  ;[1 1 1] Inputs
  (:`Started`
    (bind _possessedtdrlcharacter (`self.PossessedTDRLCharacter` :!label _label_2)
      (:`then`
        (`TDRL_Character.Input_Crouch` _possessedtdrlcharacter ActionValue)
        (if (`Character.bIsCrouched` (`GameplayStatics.GetPlayerCharacter` 0))
          (set `self.ZPlaneFloorHeight` 70.0)
          (else
            (set `self.ZPlaneFloorHeight` 145.0))))
      (:`else`)))
  (:`Canceled`
    (goto _label_2))
  (:`Completed`
    (goto _label_2)))

(event `EnhancedInput|/TopDownRogueLite/TDRL/Blueprints/Input/Actions/PrimaryAction`
  (params (ActionValue :type Boolean) (ElapsedSeconds :type "Float (double-precision)") (TriggeredSeconds :type "Float (double-precision)") (InputAction :type "InputAction Object Reference" :default "/TopDownRogueLite/TDRL/Blueprints/Input/Actions/PrimaryAction.PrimaryAction"))
  ;[1 1 1] Inputs
  (:`Started`
    (bind _possessedtdrlcharacter (`self.PossessedTDRLCharacter` :!label _label_3)
      (:`then`
        (`TDRL_Character.Input_PrimaryAction` _possessedtdrlcharacter ActionValue))
      (:`else`)))
  (:`Canceled`
    (goto _label_3))
  (:`Completed`
    (goto _label_3)))

(event `EnhancedInput|/TopDownRogueLite/TDRL/Blueprints/Input/Actions/RAction`
  (params (ActionValue :type Boolean) (ElapsedSeconds :type "Float (double-precision)") (TriggeredSeconds :type "Float (double-precision)") (InputAction :type "InputAction Object Reference" :default "/TopDownRogueLite/TDRL/Blueprints/Input/Actions/RAction.RAction"))
  ;[1 1 1] Inputs
  (:`Started`
    (bind _possessedtdrlcharacter (`self.PossessedTDRLCharacter` :!label _label_4)
      (:`then`
        (`TDRL_Character.Input_RAction` _possessedtdrlcharacter ActionValue))
      (:`else`)))
  (:`Canceled`
    (goto _label_4))
  (:`Completed`
    (goto _label_4)))

(event `EnhancedInput|/TopDownRogueLite/TDRL/Blueprints/Input/Actions/SecondaryAction`
  (params (ActionValue :type Boolean) (ElapsedSeconds :type "Float (double-precision)") (TriggeredSeconds :type "Float (double-precision)") (InputAction :type "InputAction Object Reference" :default "/TopDownRogueLite/TDRL/Blueprints/Input/Actions/SecondaryAction.SecondaryAction"))
  ;[1 1 1] Inputs
  (:`Started`
    (bind _possessedtdrlcharacter (`self.PossessedTDRLCharacter` :!label _label_5)
      (:`then`
        (`TDRL_Character.Input_SecondaryAction` _possessedtdrlcharacter ActionValue))
      (:`else`)))
  (:`Canceled`
    (goto _label_5))
  (:`Completed`
    (goto _label_5)))

(event `EnhancedInput|/TopDownRogueLite/TDRL/Blueprints/Input/Actions/PitchAim`
  (params (ActionValue :type Boolean) (ElapsedSeconds :type "Float (double-precision)") (TriggeredSeconds :type "Float (double-precision)") (InputAction :type "InputAction Object Reference" :default "/TopDownRogueLite/TDRL/Blueprints/Input/Actions/PitchAim.PitchAim"))
  ;[1 1 1] Inputs
  (:`Started`
    (bind _possessedtdrlcharacter (`self.PossessedTDRLCharacter` :!label _label_6)
      (:`then`
        (`TDRL_Character.Input_PitchAim` _possessedtdrlcharacter ActionValue))
      (:`else`)))
  (:`Canceled`
    (goto _label_6))
  (:`Completed`
    (goto _label_6)))

(event `EnhancedInput|/TopDownRogueLite/TDRL/Blueprints/Input/Actions/AlternativeWalk`
  (params (ActionValue :type Boolean) (ElapsedSeconds :type "Float (double-precision)") (TriggeredSeconds :type "Float (double-precision)") (InputAction :type "InputAction Object Reference" :default "/TopDownRogueLite/TDRL/Blueprints/Input/Actions/AlternativeWalk.AlternativeWalk"))
  ;[1 1 1] Inputs
  (:`Started`
    (bind _possessedtdrlcharacter (`self.PossessedTDRLCharacter` :!label _label_7)
      (:`then`
        (`TDRL_Character.Input_AlternativeWalk` _possessedtdrlcharacter ActionValue))
      (:`else`)))
  (:`Canceled`
    (goto _label_7))
  (:`Completed`
    (goto _label_7)))

(event `EnhancedInput|/TopDownRogueLite/TDRL/Blueprints/Input/Actions/LockTarget`
  (params (ActionValue :type Boolean) (ElapsedSeconds :type "Float (double-precision)") (TriggeredSeconds :type "Float (double-precision)") (InputAction :type "InputAction Object Reference" :default "/TopDownRogueLite/TDRL/Blueprints/Input/Actions/LockTarget.LockTarget"))
  (bind _returnvalue (`self.GetControlRotationLockedTarget`))
  (bind _returnvalue_2 (`self.GetClosestActorOfClassInRadiusUnderMouse` (`|MakeArray` "/Script/TopDownRogueLite.TDRL_Character" :!type "Actor Class Reference") 200.0 (`|MakeArray` "ObjectTypeQuery3" :!type "EObjectTypeQuery Enum") (`|MakeArray` (`self.K2_GetPawn`) :!type "Actor Object Reference") true))
  (bind _returnvalue_3 (`KismetSystemLibrary.IsValid` _returnvalue_2))
  ;[1 1 1] Inputs
  (:`Started`
    (`|ExecutionSequence`
      (:`then_0`
        (`/Engine/EditorBlueprintResources/StandardMacros.IsValid` _returnvalue
          (:`Is Valid`
            (bind _astdrl_character (cast `TDRL_Character` _returnvalue)
              (:`then`
                (remove `TDRL_Character.OnDeath` _astdrl_character (delegate `OnDeath_Event`)))
              (:`CastFailed`
                _)))
          (:`Is Not Valid`
            _))
        (`self.SetControlRotationLockedTarget` _returnvalue_2)
        (`self.SetControlRotationType` (select `bool` _returnvalue_3 :`false` "ZPlane" :`true` "LockedTarget" :!type "EControlRotationType Enum"))
        (`self.SetShouldUsePitch` _returnvalue_3)
        (set `self.bShowMouseCursor` (not _returnvalue_3))
        (if _returnvalue_3
          (bind _astdrl_character_2 (cast `TDRL_Character` _returnvalue_2))
          (add `TDRL_Character.OnDeath` _astdrl_character_2 (delegate `OnDeath_Event`))))
      (:`then_1`
        (bind _possessedtdrlcharacter (`self.PossessedTDRLCharacter` :!label _label_8)
          (:`then`
            (`TDRL_Character.Input_LockTarget` _possessedtdrlcharacter ActionValue))
          (:`else`)))))
  (:`Canceled`
    (goto _label_8))
  (:`Completed`
    (goto _label_8)))

(event `EnhancedInput|/TopDownRogueLite/TDRL/Blueprints/Input/Actions/Dash`
  (params (ActionValue :type Boolean) (ElapsedSeconds :type "Float (double-precision)") (TriggeredSeconds :type "Float (double-precision)") (InputAction :type "InputAction Object Reference" :default "/TopDownRogueLite/TDRL/Blueprints/Input/Actions/Dash.Dash"))
  ;[1 1 1] Inputs
  (:`Started`
    (bind _possessedtdrlcharacter (`self.PossessedTDRLCharacter` :!label _label_9)
      (:`then`
        (`TDRL_Character.Input_Dash` _possessedtdrlcharacter ActionValue))
      (:`else`)))
  (:`Canceled`
    (goto _label_9))
  (:`Completed`
    (goto _label_9)))

(event `OnDeath_Event`
  (params (DeathData :type "DeathData Structure"))
  ;[1 1 1] Inputs
  (if (== (`.Character` (break `DeathData` DeathData)) (`self.GetControlRotationLockedTarget`))
    (`self.SetControlRotationLockedTarget` null)
    (`self.SetControlRotationType` "ZPlane")
    (`self.SetShouldUsePitch` false)
    (set `self.bShowMouseCursor` true)))

(event `EnhancedInput|/TopDownRogueLite/TDRL/Blueprints/Input/Actions/CursorMovement`
  (params (ActionValue :type "Vector2D Structure") (ElapsedSeconds :type "Float (double-precision)") (TriggeredSeconds :type "Float (double-precision)") (InputAction :type "InputAction Object Reference" :default "/TopDownRogueLite/TDRL/Blueprints/Input/Actions/CursorMovement.CursorMovement"))
  (bind (_locationx _locationy) (`self.GetMousePosition`))
  (bind (_x _y) (`KismetMathLibrary.BreakVector2D` (* ActionValue (`self.ThumbsticCursorSpeed`))))
  ;[1 1 1] Inputs
  (:`Triggered`
    (`self.SetMouseLocation` (`KismetMathLibrary.Round` (+ _x _locationx)) (`KismetMathLibrary.Round` (+ _y _locationy)))))

(event `EnhancedInput|/TopDownRogueLite/TDRL/Blueprints/Input/Actions/NavigateGrenade`
  (params (ActionValue :type "Float (double-precision)") (ElapsedSeconds :type "Float (double-precision)") (TriggeredSeconds :type "Float (double-precision)") (InputAction :type "InputAction Object Reference" :default "/TopDownRogueLite/TDRL/Blueprints/Input/Actions/NavigateGrenade.NavigateGrenade"))
  ;[1 1 1] Inputs
  (:`Started`
    (bind _possessedtdrlcharacter (`self.PossessedTDRLCharacter`)
      (:`then`
        (`TDRL_Character.Input_NavigateGrenade` _possessedtdrlcharacter (`KismetMathLibrary.FTrunc` ActionValue)))
      (:`else`))))

(event `EnhancedInput|/TopDownRogueLite/TDRL/Blueprints/Input/Actions/ThrowGrenade`
  (params (ActionValue :type Boolean) (ElapsedSeconds :type "Float (double-precision)") (TriggeredSeconds :type "Float (double-precision)") (InputAction :type "InputAction Object Reference" :default "/TopDownRogueLite/TDRL/Blueprints/Input/Actions/ThrowGrenade.ThrowGrenade"))
  ;[1 1 1] Inputs
  (:`Started`
    (bind _possessedtdrlcharacter (`self.PossessedTDRLCharacter` :!label _label_10)
      (:`then`
        (`TDRL_Character.Input_ThrowGrenade` _possessedtdrlcharacter ActionValue))
      (:`else`)))
  (:`Canceled`
    (goto _label_10))
  (:`Completed`
    (goto _label_10)))

(event `self.PlayersSpawnAreaOverlapped`
  (params (Spawner :type "TDRL_PlayersSpawn Object Reference"))
  (`parent.PlayersSpawnAreaOverlapped` Spawner))

(event `Key|U`
  (params (Key :type "Key Structure"))
  (:`Pressed`
    (`/Engine/EditorBlueprintResources/StandardMacros.FlipFlop`
      (:`A`
        (`self.SetControlRotationType` "LockedTarget"))
      (:`B`
        (`self.SetControlRotationType` "ZPlane")))))

(event `Key|B`
  (params (Key :type "Key Structure"))
  ;[1 1 1] Respawn
  (:`Pressed`
    (`self.RespawnServer`)))

(event `RespawnServer`
  (bind _returnvalue (`GameplayStatics.GetGameMode`))
  (bind _returnvalue_2 (`GameplayStatics.GetPlayerPawn` 0))
  (bind _possessedtdrlcharacter (`self.PossessedTDRLCharacter`))
  ;[1 1 1] Respawn
  (`/Engine/EditorBlueprintResources/StandardMacros.IsValid` _possessedtdrlcharacter
    (:`Is Valid`
      (if (`TDRL_Character.GetIsDead` _possessedtdrlcharacter)
        (`/Engine/EditorBlueprintResources/StandardMacros.IsValid` _returnvalue_2 :!label _label_11
          (:`Is Valid`
            (bind _returnvalue_3 (`|SpawnActorFromClass` "/Script/AIModule.AIController" (`self.GetTransform` _returnvalue_2) "Undefined" "OverrideRootScale" null null))
            (`self.Possess` _returnvalue_3 (`GameplayStatics.GetPlayerPawn` 0)))
          (:`Is Not Valid`
            _))
        (`GameModeBase.RestartPlayerAtPlayerStart` _returnvalue self (`GameModeBase.K2_FindPlayerStart` _returnvalue self (`KismetStringLibrary.Conv_NameToString` (`self.LatestValidStartTag`))))))
    (:`Is Not Valid`
      (goto _label_11))))

(fn `LockNearestCharacter`
  (locals (L_IgnoreActors :type "Array of Actor Object Reference") (L_NearestPawn :type "Actor Object Reference") (L_NearestPawnDist :type "Float (double-precision)"))
  (bind _returnvalue (`self.K2_GetPawn`))
  (bind _returnvalue_2 (`self.K2_GetActorLocation` _returnvalue))
  (`/Engine/EditorBlueprintResources/StandardMacros.IsValid` _returnvalue ; Make sure the controller possessed a pawn
    (:`Is Valid`
      (bind _output_get (set `local.L_IgnoreActors` (`self.GetAttachedActors` _returnvalue true true))) ; Save all the attached actors (Items)
      (`KismetArrayLibrary.Array_Add` _output_get (`self.K2_GetPawn`)) ; "IgnoreSelf" will ignore the controller but not the character so add it
      (bind (_outhits _returnvalue_3) (`KismetSystemLibrary.SphereTraceMultiForObjects` _returnvalue_2 (+ _returnvalue_2 (0.0 0.0 1.0)) 300.0 (`|MakeArray` "ObjectTypeQuery3" :!type "EObjectTypeQuery Enum") false (`local.L_IgnoreActors`) "ForOneFrame"))
      (if _returnvalue_3
        ;[1 1 1] This is not needed since local variables are initialized everytime the function is called but whatever
        (set `local.L_NearestPawn` null)
        (set `local.L_NearestPawnDist` 0.0)
        (for _array_element _outhits
          (if (`KismetSystemLibrary.IsValid` (`local.L_NearestPawn`))
            (bind (_bblockinghit _binitialoverlap _time _distance _location _impactpoint _normal _impactnormal _physmat _hitactor) (`GameplayStatics.BreakHitResult` _array_element))
            (bind _returnvalue_4 (`KismetMathLibrary.Vector_Distance` _impactpoint (`self.K2_GetActorLocation` (`self.K2_GetPawn`))))
            (set `local.L_NearestPawnDist` _returnvalue_4 :!label _label)
            (set `local.L_NearestPawn` _hitactor)
            (elif (< _returnvalue_4 (`local.L_NearestPawnDist`))
              (goto _label))))
        ;[1 1 1] If the nearest actor is valid, assign it as LockedTarget and set Control Rotation Type to "LockedTarget"
        (`/Engine/EditorBlueprintResources/StandardMacros.IsValid` (`local.L_NearestPawn`)
          (:`Is Valid`
            (`self.SetControlRotationLockedTarget` (`local.L_NearestPawn`))
            (`self.SetControlRotationType` "LockedTarget")))
        (else
          ;[1 1 1] Go back to UnderMouse type
          (`self.SetControlRotationLockedTarget` null)
          (`self.SetControlRotationType` "ZPlane"))))))

(fn `UserConstructionScript`)