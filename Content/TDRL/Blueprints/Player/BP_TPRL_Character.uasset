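; Base character for players and NPCs, with possession setting up the HUD and glowstick for players or avoidance for AI.
; Input events drive GAS abilities, movement, item slots, grenade throwing and an interpolated rotate/zoom camera.
; Damage updates health, knockback and the health bar, while movement and damage report to AI perception.
; Death spawns ammo, drops items and ragdolls before destruction; debug keys teleport to checkpoints or toggle character visibility.
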(event `self.TDRL_ProgressBar.WidgetReadyOnClient`)

(event `self.ReceiveBeginPlay`
  (bind (_returnvalue_roll _returnvalue_pitch _returnvalue_yaw) (`KismetMathLibrary.BreakRotator` (`self.K2_GetActorRotation`)))
  (bind _tdrl_progressbar (`self.TDRL_ProgressBar`))
  ;[0 1 0.6833] BeginPlay
  (`self.BindUncrouchWhenFalling`)
  (set `self.CameraTargetRot` _returnvalue_yaw)
  ;[0.2396 0.1098 0.1098] Death delegate
  (add `self.OnDeath` (delegate `OnDeath_Event`))
  ;[0.2396 0.1098 0.1098] Grenade "IsThrowing" delegate
  (add `self.OnIsThrowingGrenadeChanged` (delegate `OnIsThrowingGrenadeChanged_Event`))
  ;[0 1 0.03241] Setup health bar - For multiplayer should be place after possession
  (`TDRL_ProgressBarComponent.EditProgressBarText` (`self.TDRL_ProgressBar`) "Character" (struct :`TagName` "ProgressBar.Text.Name"))
  (`TDRL_ProgressBarComponent.EditProgressBarText` _tdrl_progressbar (`KismetTextLibrary.Conv_DoubleToText` (`self.Health`) "HalfToEven" false true 1 324 0 2) (struct :`TagName` "ProgressBar.Text.Perc"))
  (`TDRL_ProgressBarComponent.EditProgressBarFloat` _tdrl_progressbar (`self.GetHealthPercentage`) (struct :`TagName` "ProgressBar.Float.Perc")))

(event `OnDeath_Event` :!signature `self.OnDeath`
  (params (DeathData :type "DeathData Structure"))
  ;[0.2396 0.1098 0.1098] Death delegate
)

(event `OnIsThrowingGrenadeChanged_Event` :!signature `self.OnIsThrowingGrenadeChanged`
  (params (NewValue :type Boolean))
  (bind (_grenadestaticdata_name _grenadestaticdata_maxarchdistance _grenadestaticdata_maxforce _grenadestaticdata_icon _grenadestaticdata_previewmesh) (break `GrenadeStaticData` (defaults `Object` (`self.GetSelectedGrenadeClass`))))
  ;[1 0.5274 0] Grenade "cosmetic" preview, replace with your own logic, socket, component etc...
  (if NewValue
    ;;[1 1 1] You can use both skeletal and static
    (bind _asstatic_mesh (cast `StaticMesh` _grenadestaticdata_previewmesh))
    (`StaticMeshComponent.SetStaticMesh` (`self.GrenadeThrowCosmetic`) _asstatic_mesh)
    (`SceneComponent.SetHiddenInGame` (`self.GrenadeThrowCosmetic`) false false)
    (else
      (`SceneComponent.SetHiddenInGame` (`self.GrenadeThrowCosmetic`) true false))))

(event `self.Input_ThrowGrenade`
  (params (bThrow :type Boolean))
  ;[1 0.5274 0] Grenade
  (if bThrow
    (`self.StartThrowingGrenade`)
    (elif (`self.IsThrowingGrenade`)
      (`self.ThrowGrenade`)
      (else
        (`self.StopThrowingGrenade`)))))

(event `self.Input_NavigateGrenade`
  (params (Positions :type Integer))
  ;[1 0.5274 0] Grenade
  (`self.SelectGrenade` (+ (`self.GetSelectedGrenadeSlot`) Positions)))

(event `self.ReceivePossessed`
  (params (NewController :type "Controller Object Reference"))
  (bind _returnvalue (`GameplayStatics.GetObjectClass` NewController))
  ;[0.2281 0.3021 0.1542] UI Possess
  (`|ExecutionSequence`
    (:`then_1`
      (if (`KismetMathLibrary.ClassIsChildOf` _returnvalue "/Script/TopDownRogueLite.TDRL_PlayerController")
        (`KismetSystemLibrary.Delay` 0.2)
        (if (`|EnumEquality` (`self.GetLocalRole`) "ROLE_Authority")
          (`self.GenUI`))
        (elif (`KismetMathLibrary.ClassIsChildOf` _returnvalue "/TopDownRogueLite/TDRL/Blueprints/AI/Controllers/BP_TDRL_NPCController_Default.BP_TDRL_NPCController_Default_C")
          (`PrimitiveComponent.SetCustomDepthStencilValue` (`self.Mesh`) 253)
          (`CharacterMovementComponent.SetAvoidanceEnabled` (`self.CharacterMovement`) true))))))

(event `GenUI`
  (bind _returnvalue (`TDRL_BFL_Global.GetTDRLHUD` self))
  ;[0.2281 0.3021 0.1542] UI Possess
  (`|ExecutionSequence`
    (:`then_0`
      (if (`self.IsLocallyControlled`)
        (`/Engine/EditorBlueprintResources/StandardMacros.IsValid` _returnvalue
          (:`Is Valid`
            (`TDRL_HUD.CreateInGameUI` _returnvalue)
            (`TDRL_HUD.SetSlotsAmount` _returnvalue (`self.InitialInventorySlots`))
            (`TDRL_HUD.RefreshIcons` _returnvalue)
            (`TDRL_HUD.SelectSlotUI` _returnvalue (`self.SelectedItemSlot`))
            (`PrimitiveComponent.SetCustomDepthStencilValue` (`self.Mesh`) 254)
            ;[1 0.5274 0] Add Grenades
            (`TDRL_GrenadePouchComponent.AddGrenadeToPouchList` (`self.GrenadePouch`) (make `GrenadePouchElement` "/TopDownRogueLite/TDRL/Blueprints/Items/Genades/BP_TDRL_Glowstick.BP_TDRL_Glowstick_C" 3))
            (`self.SelectGrenade` 0)))))))

(event `OnGrenadeThrown_Event` :!signature `self.OnGrenadeThrown`
  (params (GrenadeInstance :type "TDRL_GrenadeBase Object Reference") (TossForce :type "Vector Structure"))
  ;[1 0.5274 0] Add Grenades
)

(event `self.ReceiveRadialDamage`
  (params (DamageReceived :type "Float (single-precision)") (DamageType :type "DamageType Object Reference") (Origin :type "Vector Structure") (HitInfo :type "HitResult Structure (by ref)") (InstigatedBy :type "Controller Object Reference") (DamageCauser :type "Actor Object Reference"))
  (bind (_bblockinghit _binitialoverlap _time _distance _location _impactpoint _normal _impactnormal _physmat _hitactor _hitcomponent _hitbonename) (`GameplayStatics.BreakHitResult` HitInfo))
  ;[0.2396 0.1098 0.1098] Damage
  (`parent.ReceiveRadialDamage` DamageReceived DamageType Origin HitInfo InstigatedBy DamageCauser)
  (`self.CharacterDamaged` DamageReceived _hitbonename _impactpoint (* _impactnormal -1) InstigatedBy DamageCauser))

(event `self.ReceiveAnyDamage`
  (params (Damage :type "Float (single-precision)") (DamageType :type "DamageType Object Reference") (InstigatedBy :type "Controller Object Reference") (DamageCauser :type "Actor Object Reference"))
  ;[0.2396 0.1098 0.1098] Damage
  (`TDRL_ProgressBarComponent.SetProgressBarVisibility` (`self.TDRL_ProgressBar`) true))

(event `self.Input_Move`
  (params (Direction :type "Vector Structure"))
  (bind (_returnvalue_roll _returnvalue_pitch _returnvalue_yaw) (`KismetMathLibrary.BreakRotator` (`SceneComponent.K2_GetComponentRotation` (`self.Camera`))))
  ;[1 0.3542 0.7201] Movements
  (bind _returnvalue (`AbilitySystemComponent.TryActivateAbilitiesByTag` (`self.AbilityComponent`) (`BlueprintGameplayTagLibrary.MakeLiteralGameplayTagContainer` (struct :`GameplayTags` (struct :`(TagName` "CharacterInputs.Move")))) true))
  (if (and (not (`self.IsStunned`)) _returnvalue)
    (`self.AddMovementInput` (`KismetMathLibrary.Normal` (`KismetMathLibrary.GreaterGreater_VectorRotator` Direction (`KismetMathLibrary.MakeRotator` _returnvalue_roll 0.0 _returnvalue_yaw))))
    (`AISense_Hearing.ReportNoiseEvent` (`self.K2_GetActorLocation`) (`KismetMathLibrary.SelectFloat` 0.05 0.15 (`NavMovementComponent.IsCrouching` (`self.CharacterMovement`))) self 0.0 "AINoise")))

(event `self.Input_Crouch`
  (params (Pressed :type Boolean))
  ;[1 0.3542 0.7201] Movements
  ;;[0.8038 1 0.4115] Crouch
  (if Pressed
    (`AbilitySystemComponent.PressInputID` (`self.AbilityComponent`) (`KismetMathLibrary.Conv_ByteToInt` (enumliteral `ETDRLGASAbilityInputID` "Crouch")))))

(event `self.Death`
  (params (OutDeathData :type "DeathData Structure"))
  (bind _mesh (`self.Mesh`))
  ;[0.2396 0.1098 0.1098] Damage
  (`/Engine/EditorBlueprintResources/StandardMacros.DoOnce` false
    (:`Completed`
      (`AbilitySystemComponent.ClearAllAbilities` (`self.AbilityComponent`))
      (bind _asaicontroller (cast `AIController` (`self.GetController`))
        (:`then`
          (`AIController.RunBehaviorTree` _asaicontroller null))
        (:`CastFailed`
          _))
      (`self.DropAllItems`)
      (`PrimitiveComponent.SetCollisionResponseToChannel` (`self.CapsuleComponent`) "ECC_Pawn" "ECR_Ignore")
      (`CharacterMovementComponent.DisableMovement` (`self.CharacterMovement`))
      (`PrimitiveComponent.SetCollisionProfileName` _mesh "Ragdoll" false)
      (`PrimitiveComponent.SetSimulatePhysics` _mesh true)
      (`KismetSystemLibrary.Delay` 3.0)
      (`self.K2_DestroyActor`))))

(event `BindUncrouchWhenFalling`
  ;[1 0.3542 0.7201] Movements
  ;;[0.8038 1 0.4115] Crouch
  ;;;[1 1 1] Always UnCrouch when falling (not C++ so you can disable it if you want)
  (add `self.MovementModeChangedDelegate` (delegate `MovementModeChangedDelegate_Event`)))

(event `self.OnLanded`
  (params (Hit :type "HitResult Structure (by ref)"))
  ;[1 0.3542 0.7201] Movements
  (`AISense_Hearing.ReportNoiseEvent` (`self.K2_GetActorLocation`) 0.5 self 0.0 "AINoise"))

(event `self.Input_Dash`
  (params (Pressed :type Boolean))
  ;[1 0.3542 0.7201] Movements
  (`self.Press/ReleaseInputID` Pressed (enumliteral `ETDRLGASAbilityInputID` "Dash")))

(event `self.Input_Jump`
  (params (Pressed :type Boolean))
  ;[1 0.3542 0.7201] Movements
  (`self.Press/ReleaseInputID` Pressed (enumliteral `ETDRLGASAbilityInputID` "Jump")))

(event `MovementModeChangedDelegate_Event` :!signature `self.MovementModeChangedDelegate`
  (params (Character :type "Character Object Reference") (PrevMovementMode :type "EMovementMode Enum" :default "MOVE_None") (PreviousCustomMode :type Byte))
  (bind _charactermovement (`self.CharacterMovement`))
  ;[1 0.3542 0.7201] Movements
  ;;[0.8038 1 0.4115] Crouch
  ;;;[1 1 1] Always UnCrouch when falling (not C++ so you can disable it if you want)
  (if (and (`NavMovementComponent.IsCrouching` _charactermovement) (`|EnumEquality` (`CharacterMovementComponent.MovementMode` _charactermovement) "MOVE_Falling"))
    (`self.UnCrouch`)))

(event `self.ReceivePointDamage`
  (params (Damage :type "Float (single-precision)") (DamageType :type "DamageType Object Reference") (HitLocation :type "Vector Structure") (HitNormal :type "Vector Structure") (HitComponent :type "PrimitiveComponent Object Reference") (BoneName :type Name) (ShotFromDirection :type "Vector Structure") (InstigatedBy :type "Controller Object Reference") (DamageCauser :type "Actor Object Reference") (HitInfo :type "HitResult Structure (by ref)"))
  ;[0.2396 0.1098 0.1098] Damage
  (`parent.ReceivePointDamage` Damage DamageType HitLocation HitNormal HitComponent BoneName ShotFromDirection InstigatedBy DamageCauser HitInfo)
  (`self.CharacterDamaged` Damage BoneName HitLocation ShotFromDirection InstigatedBy DamageCauser))

(event `self.Input_AlternativeWalk`
  (params (Pressed :type Boolean))
  ;[1 0.3542 0.7201] Movements
  (`self.Press/ReleaseInputID` Pressed (enumliteral `ETDRLGASAbilityInputID` "Walk")))

(event `self.Input_PitchAim`
  (params (Pressed :type Boolean))
  ;[1 0.3542 0.7201] Movements
  (`self.Press/ReleaseInputID` Pressed (enumliteral `ETDRLGASAbilityInputID` "PitchAim")))

(event `self.Input_ChangeItemSlot`
  (params (Slot :type Byte))
  ;[0 0.5517 1] Items
  (bind _returnvalue (`AbilitySystemComponent.TryActivateAbilitiesByTag` (`self.AbilityComponent`) (`BlueprintGameplayTagLibrary.MakeLiteralGameplayTagContainer` (struct :`GameplayTags` (struct :`(TagName` "CharacterInputs.SwitchWeapon")))) true))
  (if (and _returnvalue (not (`self.IsStunned`)))
    (if (>= (`KismetArrayLibrary.Array_Length` (`self.Inventory`)) Slot)
      (`self.SelectItemSlot` Slot))))

(event `self.Input_PrimaryAction`
  (params (Pressed :type Boolean))
  ;[0 0.5517 1] Items
  ;;[1 0.75 0] Actions
  (`self.Press/ReleaseInputID` Pressed (enumliteral `ETDRLGASAbilityInputID` "PrimaryAction")))

(event `TeleportCharacter`
  (params (SpawnTag :type Name))
  (`self.TeleportChar` SpawnTag))

(event `self.Input_SecondaryAction`
  (params (Pressed :type Boolean))
  ;[0 0.5517 1] Items
  ;;[1 0.75 0] Actions
  (`self.Press/ReleaseInputID` Pressed (enumliteral `ETDRLGASAbilityInputID` "SecondaryAction")))

(event `self.Input_RotateCamera`
  (params (Value :type "Float (single-precision)"))
  ;[0.5284 0.5325 1] Snap camera rotation
  ;;[1 1 1] Smooth
  (set `self.CameraTargetRot` (`KismetMathLibrary.ClampAxis` (+ (`self.CameraTargetRot`) (* Value 1.0)))))

(event `Key|NumPadZero`
  (params (Key :type "Key Structure"))
  (:`Pressed`
    (`self.TeleportCharacter` "Start")))

(event `self.Input_Interact`
  (params (Pressed :type Boolean))
  ;[0 0.5517 1] Items
  (if Pressed
    (`AbilitySystemComponent.PressInputID` (`self.AbilityComponent`) (`KismetMathLibrary.Conv_ByteToInt` (enumliteral `ETDRLGASAbilityInputID` "Interact")))))

(event `self.Input_RAction`
  (params (Pressed :type Boolean))
  ;[0 0.5517 1] Items
  ;;[1 0.75 0] Actions
  (`self.Press/ReleaseInputID` Pressed (enumliteral `ETDRLGASAbilityInputID` "RAction")))

(event `Key|NumPadOne`
  (params (Key :type "Key Structure"))
  (:`Pressed`
    (`self.TeleportCharacter` "Checkpoint1")))

(event `self.Input_Drop`
  (params (Pressed :type Boolean))
  ;[0 0.5517 1] Items
  (if Pressed
    (`AbilitySystemComponent.PressInputID` (`self.AbilityComponent`) (`KismetMathLibrary.Conv_ByteToInt` (enumliteral `ETDRLGASAbilityInputID` "Drop")))))

(event `InputAxisKey|MouseWheelAxis`
  (params (AxisValue :type "Float (single-precision)"))
  ;[0.5284 0.5325 1] Snap camera rotation
  (if (`self.IsThrowingGrenade`)
    (`self.SetThrowingGrenadeForceMultiplier` (`KismetMathLibrary.FClamp` (+ (`self.GetThrowingGrenadeForceMultiplier`) (* AxisValue 0.01))))
    (else
      (set `self.TargetCameraDist` (`KismetMathLibrary.FClamp` (+ (* AxisValue -100.0) (`self.TargetCameraDist`)) 600.0 2000.0))
      (set `self.CameraPitch` (`KismetMathLibrary.FClamp` (+ (`self.CameraPitch`) (* AxisValue 0.05)))))))

(event `Key|NumPadTwo`
  (params (Key :type "Key Structure"))
  (:`Pressed`
    (`self.TeleportCharacter` "Checkpoint2")))

(event `Key|NumPadThree`
  (params (Key :type "Key Structure"))
  (:`Pressed`
    (`self.TeleportCharacter` "Checkpoint3")))

(event `self.ReceiveTick`
  (params (DeltaSeconds :type "Float (single-precision)"))
  (`parent.ReceiveTick` DeltaSeconds)
  (`|ExecutionSequence`
    (:`then_0`
      ;[1 1 1] Camera management
      (`self.UpdateCameraRotationAndDistance`))))

(event `Key|T`
  (params (Key :type "Key Structure"))
  (:`Pressed`
    (bind _outactors (`GameplayStatics.GetAllActorsOfClass` "/Script/TopDownRogueLite.TDRL_Character"))
    (for _array_element _outactors
      (`TDRL_BFL_Global.SetActorHiddenInGameWithAttached` _array_element))))

(event `Key|X`
  (params (Key :type "Key Structure"))
  (:`Pressed`
    (bind _outactors (`GameplayStatics.GetAllActorsOfClass` "/Script/TopDownRogueLite.TDRL_Character"))
    (for _array_element _outactors
      (`TDRL_BFL_Global.SetActorHiddenInGameWithAttached` _array_element true))))

(fn `CharacterDamaged`
  (params (Damage :type "Float (single-precision)") (Bone :type Name) (EventLocation :type "Vector Structure") (Direction :type "Vector Structure") (Instigator :type "Controller Object Reference") (Causer :type "Actor Object Reference"))
  (bind _tdrl_progressbar (`self.TDRL_ProgressBar`))
  (`AISense_Damage.ReportDamageEvent` self (`Controller.K2_GetPawn` Instigator) Damage EventLocation (0.0 0.0 0.0) "Damage")
  (`self.SetHealth` (- (`self.Health`) Damage))
  (`|ExecutionSequence`
    (:`then_0`
      (if (<= (`self.Health`) 0.0)
        (if (not (`self.GetIsDead`))
          (`self.CharacterDeath` (make `DeathData` self Causer Instigator Damage))
          (`|SpawnActorFromClass` "/TopDownRogueLite/TDRL/Blueprints/Gameplay/BP_TDRL_Ammo.BP_TDRL_Ammo_C" (`KismetMathLibrary.MakeTransform` (`NavigationSystemV1.K2_GetRandomReachablePointInRadius` (`self.K2_GetActorLocation`) 300.0 null null) (`KismetMathLibrary.MakeRotator` 0.0 0.0 (`KismetMathLibrary.RandomFloatInRange` -180.0 180.0))) "AlwaysSpawn" "OverrideRootScale" null null))))
    (:`then_1`
      ;[1 1 1] DefaultKnockback / Stun
      (`self.ApplyDefaultKnockback` Direction Bone))
    (:`then_2`
      ;[1 1 1] Update progress bar
      (`TDRL_ProgressBarComponent.EditProgressBarText` _tdrl_progressbar (`KismetTextLibrary.Conv_DoubleToText` (`self.Health`) "HalfToEven" false true 1 324 0 2) (struct :`TagName` "ProgressBar.Text.Perc"))
      (`TDRL_ProgressBarComponent.EditProgressBarFloat` _tdrl_progressbar (`self.GetHealthPercentage`) (struct :`TagName` "ProgressBar.Float.Perc")))))

(fn `PickupSpecificSlot`
  (locals (L_PreviousSlot :type Byte :default 0))
  (set `local.L_PreviousSlot` (`self.SelectedItemSlot`))
  ;[1 1 1] Select "hidden" slot for armor
  (`self.SelectItemSlot` 9)
  (`self.PickupItem` null)
  ;[1 1 1] Select "hidden" slot for armor
  (`self.SelectItemSlot` (`local.L_PreviousSlot`)))

(fn `TeleportChar`
  (params (SpawnTag :type Name))
  (locals (L_SpawnPtr :type "TDRL_PlayersSpawn Object Reference"))
  (bind _outactors (`GameplayStatics.GetAllActorsOfClass` "/Script/TopDownRogueLite.TDRL_PlayersSpawn"))
  (for _array_element _outactors
    (if (== (`TDRL_PlayersSpawn.PlayerStartTag` _array_element) SpawnTag)
      (set `local.L_SpawnPtr` _array_element)
      (break)))
  (`/Engine/EditorBlueprintResources/StandardMacros.IsValid` (`local.L_SpawnPtr`)
    (:`Is Valid`
      (`self.K2_SetActorLocation` (`NavigationSystemV1.K2_GetRandomReachablePointInRadius` (`self.K2_GetActorLocation` (`local.L_SpawnPtr`)) 100.0 null null) false true))))

(fn `TraceGrenade_Example`
  (params (LaunchVelocity :type "Vector Structure"))
  (locals (IgnoreA :type "Array of Actor Object Reference"))
  (bind _output_get (set `local.IgnoreA` (`self.GetAttachedActors` true true)))
  (`KismetArrayLibrary.Array_Insert` _output_get self)
  (`GameplayStatics.Blueprint_PredictProjectilePath_ByTraceChannel` (`SceneComponent.K2_GetComponentLocation` (`self.GrenadePivot`)) LaunchVelocity true 0.0 "ECC_Visibility" false (`local.IgnoreA`) "ForDuration" 1.0))

(fn `UpdateCameraRotationAndDistance`
  (bind _cameraspringarm (`self.CameraSpringArm`))
  (`SceneComponent.K2_SetRelativeRotation` (`self.CameraSpringArm`) (`KismetMathLibrary.RInterpTo` (`SceneComponent.RelativeRotation` (`self.CameraSpringArm`)) (`KismetMathLibrary.MakeRotator` 0.0 0.0 (`self.CameraTargetRot`)) (`GameplayStatics.GetWorldDeltaSeconds`) 18.0) false false)
  (bind _output_get (set `SpringArmComponent.TargetArmLength` (`KismetMathLibrary.FInterpTo` (`SpringArmComponent.TargetArmLength` _cameraspringarm) (`self.TargetCameraDist`) (`GameplayStatics.GetWorldDeltaSeconds`) 6.0) _cameraspringarm))
  (`SceneComponent.K2_SetRelativeLocation` _cameraspringarm (`KismetMathLibrary.MakeVector` 0.0 0.0 _output_get) false false))

(fn `UserConstructionScript`)