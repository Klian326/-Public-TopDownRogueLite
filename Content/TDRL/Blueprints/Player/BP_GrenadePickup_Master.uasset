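; Master Blueprint for grenade pickups that the player collects through interaction.
; On Interact it adds its grenade parameter to the interacting character's GrenadePouch, prints a debug "Hello" and destroys itself.
; Interaction focus toggles custom depth rendering on the static mesh for highlighting, writing a stencil value and disallowing Nanite while focused.
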(event `TDRL_InteractionInterface.Interact`
  (params (Character :type "TDRL_Character Object Reference") (Tag :type "GameplayTagContainer Structure"))
  (`KismetSystemLibrary.PrintString` "Hello")
  (`TDRL_GrenadePouchComponent.AddGrenadeToPouchList` (`TDRL_Character.GrenadePouch` Character) (`self.MyGrenadeParameter`))
  (`self.K2_DestroyActor`))

(event `TDRL_InteractionInterface.BeginInteractionFocus`
  (params (Character :type "TDRL_Character Object Reference"))
  (bind _staticmesh (`self.StaticMesh`))
  (`PrimitiveComponent.SetCustomDepthStencilValue` _staticmesh 255)
  (set `StaticMeshComponent.bDisallowNanite` true _staticmesh)
  (`PrimitiveComponent.SetRenderCustomDepth` _staticmesh true))

(event `TDRL_InteractionInterface.EndInteractionFocus`
  (params (Character :type "TDRL_Character Object Reference"))
  (bind _staticmesh (`self.StaticMesh`))
  (set `StaticMeshComponent.bDisallowNanite` false _staticmesh)
  (`PrimitiveComponent.SetRenderCustomDepth` _staticmesh false))

(fn `UserConstructionScript`)