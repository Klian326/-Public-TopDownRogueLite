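; BP_TDRL_HealthPack_S is an equippable health pack item that heals the character holding it.
; Its primary action runs the parent logic, then calls Heal on a valid equipped character with the item's heal amount and effect.
; The pack is consumed only when the heal succeeds: the character drops it and the actor destroys itself.
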(event `self.PrimaryAction`
  (params (Enabled :type Boolean))
  (bind _equippedcharacter (`self.EquippedCharacter`))
  (`parent.PrimaryAction` Enabled)
  (`/Engine/EditorBlueprintResources/StandardMacros.IsValid` _equippedcharacter
    (:`Is Valid`
      (bind _returnvalue (`TDRL_Character.Heal` _equippedcharacter (`self.HealAmount`) (`self.HealEffect`)))
      (if _returnvalue
        (`TDRL_Character.DropEquippedItem` _equippedcharacter)
        (`self.K2_DestroyActor`)))))

(fn `UserConstructionScript`
  (`parent.UserConstructionScript`))