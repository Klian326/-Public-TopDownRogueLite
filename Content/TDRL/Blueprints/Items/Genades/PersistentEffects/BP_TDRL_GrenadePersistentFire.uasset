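; Persistent fire grenade effect that deals radial falloff damage where its Niagara particles report positions.
; BeginPlay registers the actor as the Niagara collision callback, so particle data arrives locally on clients or a listen server, and dedicated servers skip tracing.
; Sphere traces keep positions near dynamic or physics-body objects and batch them into one server call to save network traffic.
; The server then applies damage at each position, credited to the instigator.
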(event `self.ReceiveBeginPlay`
  ;[1 1 1] Particle damage (Replicated)
  ;;[0 0.6366 1] Connect NiagaraSystem to this class for HitCallbacks
  (`NiagaraComponent.SetNiagaraVariableObject` (`self.BaseEffect`) "User.BPCallbackCollision" self))

(event `self.ReceiveParticleData`
  (params (Data :type "Array of BasicParticleData Structure (by ref)") (NiagaraSystem :type "NiagaraSystem Object Reference") (SimulationPositionOffset :type "Vector Structure (by ref)"))
  ;[1 1 1] Particle damage (Replicated)
  ;;[0 0 1] Receive callback locally (can be client or listen server)
  (`self.TraceForParticleDamage` Data))

(event `ApplyDamageServer`
  (params (Origins :type "Array of Vector Structure (by ref)"))
  (bind _instigator (`self.Instigator`))
  ;[1 1 1] Particle damage (Replicated)
  ;;[1 0 0] [Server] Particles damage on server
  (for _array_element Origins
    (`GameplayStatics.ApplyRadialDamageWithFalloff` :`BaseDamage` (`self.Base Damage`) :`MinimumDamage` (`self.Minimum Damage`) :`Origin` _array_element :`DamageInnerRadius` (`self.ParticleDamageMinRadius`) :`DamageOuterRadius` (`self.ParticleDamageMaxRadius`) :`DamageFalloff` (`self.Damage Falloff`) :`DamageCauser` _instigator :`InstigatedByController` (`Pawn.GetController` _instigator))))

(fn `TraceForParticleDamage`
  (params (Array :type "Array of BasicParticleData Structure"))
  (locals (L_ValidLocations :type "Array of Vector Structure"))
  (`/Engine/EditorBlueprintResources/ActorMacros.Switch Has Authority` ; Enable Clients
    (:`Authority`
      (if (not (`KismetSystemLibrary.IsDedicatedServer`))
        (for _array_element Array :!label _label
          (bind _position (break `BasicParticleData` _array_element))
          ;[1 1 1] Gather all the locations so we can send just one serialized array over the network and not multiple calls
          (bind (_outhit _returnvalue) (`KismetSystemLibrary.SphereTraceSingleForObjects` _position (+ _position (0.0 0.0 1.0)) (`self.ParticleDamageMaxRadius`) (`|MakeArray` "ObjectTypeQuery2" "ObjectTypeQuery4" :!type "EObjectTypeQuery Enum")))
          (if _returnvalue
            (`KismetArrayLibrary.Array_Add` (`local.L_ValidLocations`) _position)))
        ;[1 1 1] If there are valid locations, call for radial damage on server
        (if (> (`KismetArrayLibrary.Array_Length` (`local.L_ValidLocations`)) 0)
          (`self.ApplyDamageServer` (`local.L_ValidLocations`)))))
    (:`Remote`
      (goto _label))))

(fn `UserConstructionScript`)