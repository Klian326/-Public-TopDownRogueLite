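; Base grenade Blueprint that handles what happens when a grenade explodes.
; On the exploded event it calls the parent logic, then applies radial damage with falloff, credited to the instigator, who is excluded from the damage.
; It also applies a radial physics field through its field system at the blast location, sharing the damage's outer radius.
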(event `self.GrenadeExploded`
  (bind _returnvalue (`self.K2_GetActorLocation`))
  (bind _instigator (`self.Instigator`))
  (`parent.GrenadeExploded`)
  (`GameplayStatics.ApplyRadialDamageWithFalloff` (`self.BaseDamage`) (`self.MinimumDamage`) _returnvalue (`self.InnerRadius`) (`self.OuterRadius`) 1.0 null (`|MakeArray` _instigator :!type "Actor Object Reference") _instigator (`Pawn.GetController` _instigator))
  (`TDRL_BFL_Global.ApplyRadialFieldAtLocation` _returnvalue (make `PhysicsFieldRadialHitData` (`self.RadialFieldMagnitude`) (0.0 1.0) (`self.OuterRadius`) 0.0 "Field_FallOff_None" (`self.RadialFieldVelocity`)) (make `PhysicsFieldComponentsHitData` (`self.FieldSystem`))))

(fn `UserConstructionScript`)