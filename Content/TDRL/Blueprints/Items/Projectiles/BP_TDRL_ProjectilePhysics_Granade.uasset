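; Physics-based grenade projectile that explodes when the actor is destroyed.
; The Destroyed event spawns a Niagara explosion, applies radial damage from the projectile's static data while ignoring and crediting the owner, and plays an explosion sound.
; It also applies a reliable networked impact field at the blast point to drive Chaos destruction.
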(event `self.ReceiveDestroyed`
  (bind (_returnvalue_location _returnvalue_rotation) (`KismetMathLibrary.BreakTransform` (`self.GetTransform`)))
  (bind _returnvalue (`self.GetOwner`))
  (bind (_projectilestaticdata_instances _projectilestaticdata_trajectoryvariance _projectilestaticdata_lifetime _projectilestaticdata_damage) (break `ProjectileStaticData` (`self.ProjectileStaticData`)))
  (`NiagaraFunctionLibrary.SpawnSystemAtLocation` "/TopDownRogueLite/TDRL/DemoAssets/VisualEffects/NS_TDRL_Explosion.NS_TDRL_Explosion" _returnvalue_location _returnvalue_rotation)
  (`GameplayStatics.ApplyRadialDamage` _projectilestaticdata_damage _returnvalue_location 500.0 null (`|MakeArray` _returnvalue) self (`self.GetInstigatorController` _returnvalue))
  ;[1 0 0] Chaos Destruction
  (`self.ApplyProjectileImpactField` _returnvalue_location true)
  (`GameplayStatics.PlaySoundAtLocation` "/TopDownRogueLite/TDRL/DemoAssets/Sound/SFX/Explosion/Explosions_Grenade_Noise-Exterior-Distant_05_Cue.Explosions_Grenade_Noise-Exterior-Distant_05_Cue" (`self.K2_GetActorLocation`) (struct) 1.0 1.0 0.0 null null null null)
  (`self.K2_DestroyActor`))

(fn `UserConstructionScript`)