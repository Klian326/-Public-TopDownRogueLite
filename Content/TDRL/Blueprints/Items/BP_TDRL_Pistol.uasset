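; Pistol item for TDRL that fires, attacks on secondary action, reloads, outlines on focus and shows a Niagara laser sight.
; Equipping by a player opens a Tick gate driving UpdateLaser; dropping or holstering closes it.
; UpdateLaser sets the beam end per controller rotation mode, blending Z-plane traces near the character, and replicates it via OnRep.
; The example pitch-aim bindings are not connected.
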(event `Key|H`
  (params (Key :type "Key Structure")))

(event `TDRL_InteractionInterface.BeginInteractionFocus`
  (params (Character :type "TDRL_Character Object Reference"))
  ;[1 0 0] Item focus interaction exposed using interface
  (`self.EnableItemOutliner` true))

(event `TDRL_InteractionInterface.EndInteractionFocus`
  (params (Character :type "TDRL_Character Object Reference"))
  ;[1 0 0] Item focus interaction exposed using interface
  (`self.EnableItemOutliner` false))

(event `self.PrimaryAction`
  (params (Enabled :type Boolean))
  (`parent.PrimaryAction` Enabled)
  (if Enabled
    (`self.StartFiring`)
    (elif (not (> (`.Burst` (break `FirearmStaticData` (`self.FirearmStaticData`))) 0))
      (`self.StopFiring`))))

(event `self.ReceiveBeginPlay`
  (`self.AddDamageBody` (`self.Capsule1`))
  ;[1 1 1] Laser
  (add `self.OnEquip` (delegate `CustomEvent`))
  (add `self.OnDrop` (delegate `HideLaser`))
  (add `self.OnHolster` (delegate `HideLaser`)))

(event `self.SecondaryAction`
  (params (Enabled :type Boolean))
  (`parent.PrimaryAction` Enabled)
  (if Enabled
    (`self.StartAttack`)
    (else
      (`self.StopAttack`))))

(event `HideLaser`
  (params (InteractingCharacter :type "TDRL_Character Object Reference"))
  ;[1 1 1] Laser
  (`SceneComponent.SetVisibility` (`self.Niagara`) false false)
  (goto _label :!via `Close`))

(event `CustomEvent` :!signature `self.OnEquip`
  (params (InteractingCharacter :type "TDRL_Character Object Reference"))
  ;[1 1 1] Laser
  (if (`Pawn.IsPlayerControlled` InteractingCharacter)
    (set `self.OwnerController` (`TDRL_Character.GetOwningPlayerController_TDRL` InteractingCharacter))
    (`SceneComponent.SetVisibility` (`self.Niagara`) true false)
    (goto _label :!via `Open`)))

(event `self.RAction`
  (params (Enabled :type Boolean))
  (`parent.RAction` Enabled)
  (if Enabled
    (`self.ReloadWeapon`)))

(event `self.ReceiveTick`
  (params (DeltaSeconds :type "Float (single-precision)"))
  ;[1 1 1] Laser
  (`/Engine/EditorBlueprintResources/StandardMacros.Gate` true :!label _label
    (:`Exit`
      (`self.UpdateLaser`))))

(event `ReplicateLaserEnd`
  (params (LaserEnd :type "Vector Structure"))
  ;[1 1 1] Laser
  (set `self.Laser End Replicated` LaserEnd))

(event `OnEquip_Event` :!signature `self.OnEquip`
  (params (InteractingCharacter :type "TDRL_Character Object Reference"))
  ;[1 0.7396 0] [Example] Enable pitchaim when equipping this class, disable pitchaim if it's holstered or if it's dropped
  (`TDRL_Character.Input_PitchAim` InteractingCharacter true))

(event `OnHolster_Event` :!signature `self.OnHolster`
  (params (InteractingCharacter :type "TDRL_Character Object Reference"))
  ;[1 0.7396 0] [Example] Enable pitchaim when equipping this class, disable pitchaim if it's holstered or if it's dropped
  (`TDRL_Character.Input_PitchAim` InteractingCharacter false))

(event `OnDrop_Event` :!signature `self.OnDrop`
  (params (InteractingCharacter :type "TDRL_Character Object Reference"))
  ;[1 0.7396 0] [Example] Enable pitchaim when equipping this class, disable pitchaim if it's holstered or if it's dropped
  (if (== (`TDRL_Character.GetEquippedItem` InteractingCharacter) self)
    (`TDRL_Character.Input_PitchAim` InteractingCharacter false)))

(fn `GetOwnerFeetLocation`
  (returns (ReturnValue :type "Vector Structure"))
  (bind _equippedcharacter (`self.EquippedCharacter`))
  (return (- (`self.K2_GetActorLocation` _equippedcharacter) (`KismetMathLibrary.MakeVector` 0.0 0.0 (`CapsuleComponent.GetScaledCapsuleHalfHeight` (`Character.CapsuleComponent` _equippedcharacter))))))

(fn `OnRep_Laser End Replicated`
  (`FXSystemComponent.SetVectorParameter` (`self.Niagara`) "BeamEnd" (`self.Laser End Replicated`)))

(fn `UpdateLaser`
  (locals (L_IgnoreActors :type "Array of Actor Object Reference") (L_TargetEnd :type "Vector Structure" :default (0.0 0.0 0.0)))
  (bind _equippedcharacter (`self.EquippedCharacter`))
  (bind _ownercontroller (`self.OwnerController`))
  (bind _returnvalue (`TDRL_PlayerController.GetControlRotationLockedTarget` _ownercontroller))
  (bind _returnvalue_2 (`SceneComponent.K2_GetComponentLocation` (`self.Niagara`)))
  (bind _returnvalue_3 (`SceneComponent.K2_GetComponentLocation` (`self.Niagara`)))
  (bind _deadzonearoundcharacter (`TDRL_PlayerController.DeadZoneAroundCharacter` (`self.OwnerController`)))
  (bind _returnvalue_4 (/ _deadzonearoundcharacter 2.0))
  (bind _returnvalue_5 (`KismetMathLibrary.MapRangeClamped` (`KismetMathLibrary.Vector_Distance2D` (`TDRL_PlayerController.ZPlaneTargetLocation` (`self.OwnerController`)) (`self.K2_GetActorLocation` (`self.EquippedCharacter`))) (- _deadzonearoundcharacter _returnvalue_4) (+ _deadzonearoundcharacter _returnvalue_4) 1.0))
  (bind _returnvalue_6 (`KismetMathLibrary.VLerp` _returnvalue_2 (+ (`self.GetOwnerFeetLocation`) (`KismetMathLibrary.MakeVector` 0.0 0.0 (`TDRL_PlayerController.ZPlaneFloorHeight` (`self.OwnerController`)))) _returnvalue_5))
  (if (and (`KismetSystemLibrary.IsValid` (`self.OwnerController`)) (`KismetSystemLibrary.IsValid` _equippedcharacter))
    (if (`Pawn.IsLocallyControlled` _equippedcharacter)
      (bind _output_get (set `local.L_IgnoreActors` (`self.GetAttachedActors` (`self.GetAttachParentActor`) true false)))
      (`KismetArrayLibrary.Array_Add` _output_get (`self.GetAttachParentActor`))
      (switch `EControlRotationType` (`TDRL_PlayerController.GetControlRotationType` (`self.OwnerController`))
        (:`ZPlane`
          (bind (_outhit _returnvalue_7) (`KismetSystemLibrary.LineTraceSingle` _returnvalue_6 (+ _returnvalue_6 (* (`KismetMathLibrary.VLerp` (`KismetMathLibrary.GetDirectionUnitVector` _returnvalue_2 (`TDRL_PlayerController.ZPlaneTargetLocation` (`self.OwnerController`))) (`KismetMathLibrary.GetForwardVector` (`Controller.GetControlRotation` (`self.OwnerController`))) _returnvalue_5) 50000000000000.0)) "TraceTypeQuery1" false (`local.L_IgnoreActors`) "None" true (struct :`G` 0.500689 :`B` 1.0 :`A` 1.0) (struct :`G` 1.0 :`A` 1.0) 0.1 :!label _label))
          (bind (_bblockinghit _binitialoverlap _time _distance _location _impactpoint _normal _impactnormal _physmat _hitactor _hitcomponent _hitbonename _bonename _hititem _elementindex _faceindex _tracestart _traceend) (`GameplayStatics.BreakHitResult` _outhit))
          (set `local.L_TargetEnd` (`KismetMathLibrary.SelectVector` _impactpoint _traceend _returnvalue_7)))
        (:`LockedTarget`
          (`/Engine/EditorBlueprintResources/StandardMacros.IsValid` _returnvalue
            (:`Is Valid`
              (set `local.L_TargetEnd` (`self.K2_GetActorLocation` _returnvalue)))
            (:`Is Not Valid`
              (goto _label))))
        (:`TargetLocation`
          (set `local.L_TargetEnd` (`TDRL_PlayerController.GetControlRotationTargetLocation` _ownercontroller)))
        (:`WorldRotation`
          (bind (_outhit_2 _returnvalue_8) (`KismetSystemLibrary.LineTraceSingle` _returnvalue_3 (+ _returnvalue_3 (* (`KismetMathLibrary.GetForwardVector` (`Controller.GetControlRotation` (`self.OwnerController`))) 5000000.0)) "TraceTypeQuery1" false (`local.L_IgnoreActors`) "None" true (struct :`G` 0.500689 :`B` 1.0 :`A` 1.0) (struct :`G` 1.0 :`A` 1.0) 0.1))
          (bind (_bblockinghit_2 _binitialoverlap_2 _time_2 _distance_2 _location_2 _impactpoint_2 _normal_2 _impactnormal_2 _physmat_2 _hitactor_2 _hitcomponent_2 _hitbonename_2 _bonename_2 _hititem_2 _elementindex_2 _faceindex_2 _tracestart_2 _traceend_2) (`GameplayStatics.BreakHitResult` _outhit_2))
          (set `local.L_TargetEnd` (`KismetMathLibrary.SelectVector` _impactpoint_2 _traceend_2 _returnvalue_8))))
      (`self.ReplicateLaserEnd` (`local.L_TargetEnd`))
      (`FXSystemComponent.SetVectorParameter` (`self.Niagara`) "BeamEnd" (`local.L_TargetEnd`)))))

(fn `UserConstructionScript`)