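; BP_TDRL_Flag_01 is a flag item that the player can focus on and use to attack.
; Gaining or losing interaction focus through the interface toggles the item's outline highlight.
; On BeginPlay it registers Capsule1 as a damage body.
; Its primary action calls the parent implementation, then starts the attack when enabled and stops it when released.
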(event `TDRL_InteractionInterface.BeginInteractionFocus`
  (params (Character :type "TDRL_Character Object Reference"))
  ;[1 0 0] Item focus interaction exposed using interface
  (`self.EnableItemOutliner` true))

(event `TDRL_InteractionInterface.EndInteractionFocus`
  (params (Character :type "TDRL_Character Object Reference"))
  ;[1 0 0] Item focus interaction exposed using interface
  (`self.EnableItemOutliner` false))

(event `self.ReceiveBeginPlay`
  (`self.AddDamageBody` (`self.Capsule1`)))

(event `self.PrimaryAction`
  (params (Enabled :type Boolean))
  (`parent.PrimaryAction` Enabled)
  (if Enabled
    (`self.StartAttack`)
    (else
      (`self.StopAttack`))))

(fn `UserConstructionScript`)