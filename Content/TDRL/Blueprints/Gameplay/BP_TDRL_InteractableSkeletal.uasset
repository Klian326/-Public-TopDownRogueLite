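; Base-style interactable skeletal mesh actor that highlights on focus and responds to a single interaction, apparently as a lever.
; Focus begin and end events toggle custom depth rendering on the skeletal mesh.
; Interact, noted as server-side via GA_Pickup, passes a DoOnce that is never reset, flips the LeverEnbaled flag and calls Interacted.
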(event `TDRL_InteractionInterface.BeginInteractionFocus`
  (params (Character :type "TDRL_Character Object Reference"))
  (`PrimitiveComponent.SetRenderCustomDepth` (`self.SkeletalMeshComponent`) true))

(event `TDRL_InteractionInterface.EndInteractionFocus`
  (params (Character :type "TDRL_Character Object Reference"))
  (`PrimitiveComponent.SetRenderCustomDepth` (`self.SkeletalMeshComponent`) false))

(event `TDRL_InteractionInterface.Interact`
  (params (Character :type "TDRL_Character Object Reference") (Tag :type "GameplayTagContainer Structure"))
  ;[1 1 1] On server. Check GA_Pickup
  (`/Engine/EditorBlueprintResources/StandardMacros.DoOnce` false
    (:`Completed`
      (set `self.bLeverEnbaled` (not (`self.bLeverEnbaled`)))
      ;;[0 0 1] Blueprint
      (`self.Interacted`))))

(fn `UserConstructionScript`)