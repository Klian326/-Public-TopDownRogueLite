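; Example occludable static mesh actor that fades when the TDRL camera occlusion component reports it blocks the camera.
; BeginPlay creates a dynamic material for slot 0 and registers the mesh as the affected component.
; Occlusion changes toggle the mesh's Visibility trace response and play or reverse a timeline driving the Opacity parameter, which needs a translucent or masked material.
; The default hide/unhide call is left unconnected as an alternative.
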(event `self.ReceiveBeginPlay`
  (bind _staticmeshcomponent (`self.StaticMeshComponent`))
  ;[1 1 1] Create and apply dynamic material
  (bind _returnvalue (`PrimitiveComponent.CreateDynamicMaterialInstance` _staticmeshcomponent 0 (`PrimitiveComponent.GetMaterial` _staticmeshcomponent 0) "None"))
  (bind _output_get (set `self.FadeMaterial` _returnvalue))
  (`PrimitiveComponent.SetMaterial` (`self.StaticMeshComponent`) 0 _output_get)
  ;[1 1 1] Set affected component
  (`TDRL_CameraOcclusionComponent.SetAffectedComponents` (`self.TDRL_CameraOcclusion`) (`|MakeArray` (`self.StaticMeshComponent`) :!type "PrimitiveComponent Object Reference")))

(event `self.TDRL_CameraOcclusion.OnOcclusionChanged`
  (params (Occluded :type Boolean) (OcclusionComps :type "Array of SceneComponent Object Reference"))
  ;[1 1 1] Fade setup example (will need translucient o masked material)
  (`PrimitiveComponent.SetCollisionResponseToChannel` (`self.StaticMeshComponent`) "ECC_Visibility" (select `bool` Occluded :`false` "ECR_Block" :`true` "ECR_Ignore" :!type "ECollisionResponse Enum"))
  (if Occluded
    (bind (_direction _visibility) (`Timeline|FadeMesh` :!label _label)
      (:`Update`
        (`MaterialInstanceDynamic.SetScalarParameterValue` (`self.FadeMaterial`) "Opacity" _visibility)))
    (else
      (goto _label :!via `Reverse`))))

(fn `UserConstructionScript`)