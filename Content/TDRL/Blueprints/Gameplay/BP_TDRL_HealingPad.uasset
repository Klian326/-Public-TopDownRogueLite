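; Healing pad actor that heals a TDRL_Character entering its box, then recharges before it can heal again.
; A dynamic glow material on the mesh switches between ready and charging colors to show its state.
; A DoOnce gates overlaps during recharge, after which the first character still inside is healed and the cycle repeats.
; The gate resets when a heal fails or the pad is empty after recharging.
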(event `self.ReceiveBeginPlay`
  ;[1 1 1] Dynamic Material
  (bind _returnvalue (`PrimitiveComponent.CreateDynamicMaterialInstance` (`self.StaticMesh`) 0 "/TopDownRogueLite/TDRL/DemoAssets/Materials/Items/MI_TDRL_InternalShapeGlow_Hex.MI_TDRL_InternalShapeGlow_Hex" "None"))
  (bind _output_get (set `self.CurDynMat` _returnvalue))
  (`PrimitiveComponent.SetMaterial` (`self.StaticMesh`) 0 _output_get)
  (`MaterialInstanceDynamic.SetVectorParameterValue` (`self.CurDynMat`) "Color" (`self.ReadyColor`)))

(event `self.Box.OnComponentBeginOverlap`
  (params (OverlappedComponent :type "PrimitiveComponent Object Reference") (OtherActor :type "Actor Object Reference") (OtherComp :type "PrimitiveComponent Object Reference") (OtherBodyIndex :type Integer) (bFromSweep :type Boolean) (SweepResult :type "HitResult Structure (by ref)"))
  (bind _overlappingactors (`PrimitiveComponent.GetOverlappingActors` (`self.Box`) "/Script/TopDownRogueLite.TDRL_Character"))
  ;[1 1 1] Overlap
  (bind _astdrl_character (cast `TDRL_Character` OtherActor))
  (`/Engine/EditorBlueprintResources/StandardMacros.DoOnce` false :!label _label
    (:`Completed`
      (bind _returnvalue (`TDRL_Character.Heal` _astdrl_character (`self.HealAmount`) (`self.HealEffects`)))
      (if _returnvalue
        (`MaterialInstanceDynamic.SetVectorParameterValue` (`self.CurDynMat`) "Color" (`self.ChargingColor`) :!label _label_2)
        (`KismetSystemLibrary.Delay` (`self.RechargeTime`))
        (`MaterialInstanceDynamic.SetVectorParameterValue` (`self.CurDynMat`) "Color" (`self.ReadyColor`))
        (if (> (`KismetArrayLibrary.Array_Length` _overlappingactors) 0)
          (bind _returnvalue_2 (`TDRL_Character.Heal` (cast `TDRL_Character` (`|GetArrayItem` _overlappingactors) :!pure true) (`self.HealAmount`) (`self.HealEffects`)))
          (if _returnvalue_2
            (goto _label_2)
            (else
              (goto _label :!via `Reset`)))
          (else
            (goto _label :!via `Reset`)))
        (else
          (goto _label :!via `Reset`))))))

(fn `UserConstructionScript`)