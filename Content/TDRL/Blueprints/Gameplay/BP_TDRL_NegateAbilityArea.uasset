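; BP_TDRL_NegateAbilityArea is a box volume that takes configured abilities away from any TDRL_Character inside it.
; On overlap begin, it loops over the AbilityClass array and clears all abilities on the character's AbilityComponent bound to each class's default input ID.
; On overlap end, it grants each listed class at level 1 on that input, without checking what the character had before.
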(event `self.Box.OnComponentBeginOverlap`
  (params (OverlappedComponent :type "PrimitiveComponent Object Reference") (OtherActor :type "Actor Object Reference") (OtherComp :type "PrimitiveComponent Object Reference") (OtherBodyIndex :type Integer) (bFromSweep :type Boolean) (SweepResult :type "HitResult Structure (by ref)"))
  (bind _astdrl_character (cast `TDRL_Character` OtherActor))
  (for _array_element (`self.Ability Class`)
    (if (`KismetSystemLibrary.IsValidClass` _array_element)
      (`AbilitySystemComponent.ClearAllAbilitiesWithInputID` (`TDRL_Character.AbilityComponent` _astdrl_character) (`KismetMathLibrary.Conv_ByteToInt` (defaults `Object` _array_element))))))

(event `self.Box.OnComponentEndOverlap`
  (params (OverlappedComponent :type "PrimitiveComponent Object Reference") (OtherActor :type "Actor Object Reference") (OtherComp :type "PrimitiveComponent Object Reference") (OtherBodyIndex :type Integer))
  (bind _astdrl_character (cast `TDRL_Character` OtherActor))
  (for _array_element (`self.Ability Class`)
    (if (`KismetSystemLibrary.IsValidClass` _array_element)
      (`AbilitySystemComponent.K2_GiveAbility` (`TDRL_Character.AbilityComponent` _astdrl_character) _array_element 1 (`KismetMathLibrary.Conv_ByteToInt` (defaults `Object` _array_element))))))

(fn `UserConstructionScript`
  (`parent.UserConstructionScript`))