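; Default AI controller for TDRL NPCs that turns perception stimuli into alert and blackboard state.
; On possess it resets the alert state, then after a short delay picks a mobility state based on whether a PatrolTarget is set.
; Perceived living player characters become the alert threat, while noise stimuli can raise alertness and record the sound location in the blackboard.
; Timers manage lowering the alert level, refreshed when the current threat is perceived again.
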(event `self.ReceivePossess`
  (params (PossessedPawn :type "Pawn Object Reference"))
  (bind _returnvalue (`AIBlueprintHelperLibrary.GetBlackboard` null))
  ;[1 0 0] Possess
  (`/Engine/EditorBlueprintResources/StandardMacros.IsValid` _returnvalue
    (:`Is Valid`
      (`BlackboardComponent.SetValueAsEnum` _returnvalue "AlertState" (enumliteral `/TopDownRogueLite/TDRL/Blueprints/AI/Behaviours/Enum_NPCAlertState` "NewEnumerator0"))
      (`KismetSystemLibrary.Delay` 0.5)
      (`BlackboardComponent.SetValueAsEnum` _returnvalue "MobilityState" (select `bool` (`KismetSystemLibrary.IsValid` (`BlackboardComponent.GetValueAsObject` (`AIBlueprintHelperLibrary.GetBlackboard` null) "PatrolTarget")) :`false` (enumliteral `/TopDownRogueLite/TDRL/Blueprints/AI/Behaviours/Enum_NPCMobilityState` "NewEnumerator2") :`true` (enumliteral `/TopDownRogueLite/TDRL/Blueprints/AI/Behaviours/Enum_NPCMobilityState` "NewEnumerator1") :!type "Byte")))))

(event `self.Perception.OnTargetPerceptionUpdated`
  (params (Actor :type "Actor Object Reference") (Stimulus :type "AIStimulus Structure"))
  (bind (_age _expirationage _strength _stimuluslocation _receiverlocation _tag) (break `AIStimulus` Stimulus))
  (bind _returnvalue (`AIBlueprintHelperLibrary.GetBlackboard` null))
  ;[0 0.09559 1] AI (NPCController)
  (if (!= self Actor)
    (`|ExecutionSequence`
      (:`then_0`
        (switch `name` _tag
          (:`Default`
            (bind _astdrl_character (cast `TDRL_Character` Actor))
            (if (`TDRL_Character.GetIsDead` _astdrl_character)
              _
              (elif (== _astdrl_character (`self.GetAlertThreat`))
                (`self.RefreshReduceAlertLevelWithTimer`)
                (elif (`Pawn.IsPlayerControlled` _astdrl_character)
                  (`self.SetAlertState` (enumliteral `/TopDownRogueLite/TDRL/Blueprints/AI/Behaviours/Enum_NPCAlertState` "NewEnumerator2"))
                  (`self.EnableReduceAlertLevelWithTimer` true)
                  (`self.SetAlertThreat` _astdrl_character)))))
          (:`AINoise`
            (if (== (`self.GetAlertState`) (enumliteral `/TopDownRogueLite/TDRL/Blueprints/AI/Behaviours/Enum_NPCAlertState` "NewEnumerator0")) :!label _label
              (`|ExecutionSequence`
                (:`then_0`
                  (`self.SetAlertState` (enumliteral `/TopDownRogueLite/TDRL/Blueprints/AI/Behaviours/Enum_NPCAlertState` "NewEnumerator1"))
                  (`self.EnableReduceAlertLevelWithTimer` true))
                (:`then_1`
                  ;;[1 1 1] Non C++ using your own custom blackboard variables
                  (`/Engine/EditorBlueprintResources/StandardMacros.IsValid` _returnvalue :!label _label_2
                    (:`Is Valid`
                      (`BlackboardComponent.SetValueAsBool` _returnvalue "SusSoundToCheck" true)
                      (`BlackboardComponent.SetValueAsVector` _returnvalue "SusLastSoundHearedLocation" _stimuluslocation)))))
              (else
                (goto _label_2))))
          (:`AINoiseHit`
            (goto _label)))))))

(event `self.Perception.OnPerceptionUpdated`
  (params (UpdatedActors :type "Array of Actor Object Reference (by ref)"))
  ;[0 0.09559 1] AI (NPCController)
)

(fn `UserConstructionScript`)